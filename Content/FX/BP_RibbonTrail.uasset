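; BP_RibbonTrail is an FX actor that moves itself along a weaving path, likely to drive or showcase a ribbon trail.
; Tick offsets it along its forward vector by MoveSpeed, scaled by delta time and without sweeping.
; A looping one-second timer negates the RotatingMovement component's yaw rate, so the heading swings back and forth as it travels.
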(event `self.ReceiveBeginPlay`
  (`KismetSystemLibrary.K2_SetTimer` null "RotationSwitch" 1.0 true))

(event `self.ReceiveTick`
  (params (DeltaSeconds :type "Float (single-precision)"))
  (`self.K2_AddActorWorldOffset` (* (`self.GetActorForwardVector`) (* DeltaSeconds (`self.MoveSpeed`)))))

(event `RotationSwitch`
  (bind (_rotationrate_roll _rotationrate_pitch _rotationrate_yaw) (`KismetMathLibrary.BreakRotator` (`RotatingMovementComponent.RotationRate` (`self.RotatingMovement`))))
  (set `RotatingMovementComponent.RotationRate` (`KismetMathLibrary.MakeRotator` 0.0 0.0 (* _rotationrate_yaw -1.0)) (`self.RotatingMovement`)))

(fn `UserConstructionScript`)